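; BP_FlyArea is an actor that fills an axis-aligned box around its location with an evenly spaced 3D grid of position nodes.
; The construction script derives the box extents from BoxScale and draws debug spheres at its eight corners.
; On BeginPlay, spacing comes from the per-axis node count, and CreateNodesInFlyArea fills NodeArray, looping along X and recursing for Y and Z.
; Debug prints timestamp the build, then boxes mark each node.
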(event EventBeginPlay
  (CallFunction|GetSpacingBetweenNodes)
  (CallFunction|SetMinMaxExtents)
  (Utilities|Array|Clear (Variables|Default|GetNodeArray))
  (Variables|Default|SetNextNodePosition (Variables|Default|GetMinExtents))
  (Development|PrintString (Utilities|String|Append (Utilities|GetDisplayName self) (Utilities|String|ToString(Float) (Utilities|Time|GetGameTimeinSeconds)) "Before"))
  (CallFunction|CreateNodesinFlyArea)
  (Development|PrintString (Utilities|String|Append (Utilities|String|ToString(Float) (Utilities|Time|GetGameTimeinSeconds)) (Utilities|GetDisplayName self) "After"))
  (for _array_element (Variables|Default|GetNodeArray)
    (Rendering|Debug|DrawDebugBox (.NodePosition (Utilities|Struct|BreakS_PositionNodeBP _array_element)) "20.000000,20.000000,20.000000" "(R=0.014317,G=0.105290,B=1.000000,A=1.000000)" "0, 0, 0" 1e+01 5.0)))

(event Collision|EventActorBeginOverlap
  (params (OtherActor :type Actor%20Object%20Reference)))

(event EventTick
  (params (DeltaSeconds :type Float%20%28single-precision%29)))

(fn ConstructionScript
  (bind _maxextents (Variables|Default|GetMaxExtents))
  (bind _minextents (Variables|Default|GetMinExtents))
  (bind _maxextents_2 (Variables|Default|GetMaxExtents))
  (bind _minextents_2 (Variables|Default|GetMinExtents))
  (Utilities|Array|Clear (Variables|Default|GetNodeArray))
  (Utilities|Array|Clear (Variables|Default|GetCorners))
  (CallFunction|SetMinMaxExtents)
  (bind _output_get (Variables|Default|SetCorners (Utilities|Array|MakeArray (Math|Vector|MakeVector (.x _minextents_2) (.y _maxextents_2) (.z _maxextents_2)) (Math|Vector|MakeVector (.x _maxextents_2) (.y _minextents_2) (.z _maxextents_2)) (Math|Vector|MakeVector (.x _maxextents_2) (.y _maxextents_2) (.z _minextents_2)) (Math|Vector|MakeVector (.x _maxextents) (.y _minextents) (.z _minextents)) (Math|Vector|MakeVector (.x _minextents) (.y _maxextents) (.z _minextents)) (Math|Vector|MakeVector (.x _minextents) (.y _minextents) (.z _maxextents)) (Variables|Default|GetMinExtents) (Variables|Default|GetMaxExtents))))
  (for _array_element _output_get
    (Rendering|Debug|DrawDebugSphere _array_element 1e+02 12 "(R=1.000000,G=0.000000,B=0.117538,A=1.000000)" 3e+01 1e+01)))

(fn SetMinMaxExtents
  (bind _returnvalue (Transformation|GetActorLocation))
  (bind _boxscale (Variables|Default|GetBoxScale))
  (bind _returnvalue_2 (/ _boxscale 2.0))
  (Variables|Default|SetMaxExtents (+ _returnvalue _returnvalue_2))
  (Variables|Default|SetMinExtents (Math|Vector|NegateVector (- _returnvalue_2 _returnvalue))))

(fn GetSpacingBetweenNodes
  (Variables|Default|SetSpacingBetweenNodes (Math|Vector|VectorGetAbs (/ (Variables|Default|GetBoxScale) (- (Variables|Default|GetNodesRequiredForEachAxis) 1)))))

(fn CreateNodesinFlyArea
  (bind _minextents (Variables|Default|GetMinExtents))
  (while (<= (.x (Variables|Default|GetNextNodePosition)) (.x (Variables|Default|GetMaxExtents)))
    (Utilities|Array|Add (Variables|Default|GetNodeArray) (Utilities|Struct|MakeS_PositionNodeBP true (Variables|Default|GetNextNodePosition)))
    (Variables|Default|SetNextNodePosition (Math|Vector|MakeVector (+ (.x (Variables|Default|GetNextNodePosition)) (.x (Variables|Default|GetSpacingBetweenNodes))) (.y (Variables|Default|GetNextNodePosition)) (.z (Variables|Default|GetNextNodePosition)))))
  (Variables|Default|SetNextNodePosition (Math|Vector|MakeVector (.x (Variables|Default|GetMinExtents)) (+ (.y (Variables|Default|GetSpacingBetweenNodes)) (.y (Variables|Default|GetNextNodePosition))) (.z (Variables|Default|GetNextNodePosition))))
  (if (<= (.y (Variables|Default|GetNextNodePosition)) (.y (Variables|Default|GetMaxExtents)))
    (CallFunction|CreateNodesinFlyArea)
    (else
      (Variables|Default|SetNextNodePosition (Math|Vector|MakeVector (.x _minextents) (.y _minextents) (+ (.z (Variables|Default|GetSpacingBetweenNodes)) (.z (Variables|Default|GetNextNodePosition)))))
      (if (<= (.z (Variables|Default|GetNextNodePosition)) (.z (Variables|Default|GetMaxExtents)))
        (CallFunction|CreateNodesinFlyArea)))))